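; Live Link remap asset that adjusts incoming curve names and values, apparently for facial animation.
; GetRemappedCurveName prefixes each curve name with "face." for the target.
; RemapCurveElements runs each curve value through a smoothstep math expression (3x² − 2x³).
; Its results are written under the key "None" rather than the looped curve's name, so the original entries keep their values.
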(fn GetRemappedCurveName
  (params (CurveName :type Name :default "None"))
  (return (Utilities|String|StringToName (Utilities|String|Append "face." (Utilities|String|ToString(Name) CurveName)))))

(fn RemapCurveElements
  (params (CurveItems :type Map%20of%20Names%20to%20Reals))
  (bind _keys (Utilities|Map|Keys CurveItems))
  (for _array_element _keys
    (Utilities|Map|Add CurveItems "" (|(((3*x)*x)-(((2*x)*x)*x)) (.Value (Utilities|Map|Find CurveItems _array_element)))))
  (return))