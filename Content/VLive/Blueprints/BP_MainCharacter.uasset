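; BP_MainCharacter is the VLive main character blueprint, carrying a cine camera and directional light rig that it positions on BeginPlay.
; SetComponentTransform sets the camera's arm length, offset, yaw and pitch, the Scene component's yaw, and the light's rotation.
; It then derives the manual focus distance from the camera's relative distance to a fixed raised point, likely head height, so focus follows the framing.
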(event `self.ReceiveBeginPlay`
  (`self.SetComponentTransform` 200.0 0.0 (0.0 120.0 0.0) 0.0 0.0 (struct :`Pitch` -30.0 :`Yaw` 30.0)))

(fn `SetComponentTransform`
  (params (ArmLength :type "Float (double-precision)") (ArmAngle :type "Float (double-precision)") (CamPos :type "Vector Structure") (CamYaw :type "Float (double-precision)") (CamPitch :type "Float (double-precision)") (LightRotation :type "Rotator Structure"))
  (bind (_campos_x _campos_y) (`KismetMathLibrary.BreakVector` (`local.CamPos`)))
  (bind _cinecamera (`self.CineCamera`))
  (bind (_focussettings_focusmethod _focussettings_manualfocusdistance _focussettings_trackingfocussettings _focussettings_bsmoothfocuschanges _focussettings_focussmoothinginterpspeed _focussettings_focusoffset) (break `CameraFocusSettings` (`CineCameraComponent.FocusSettings` _cinecamera)))
  (`SceneComponent.K2_SetRelativeTransform` (`self.CineCamera`) (`KismetMathLibrary.MakeTransform` (`KismetMathLibrary.MakeVector` (* (`local.ArmLength`) -1.0) _campos_x _campos_y) (`KismetMathLibrary.MakeRotator` 0.0 (`local.CamPitch`) (`local.CamYaw`))) false true)
  (`SceneComponent.K2_SetRelativeRotation` (`self.Scene`) (`KismetMathLibrary.MakeRotator` 0.0 0.0 (`local.ArmAngle`)) false true)
  (`SceneComponent.K2_SetRelativeRotation` (`self.DirectionalLight`) (`local.LightRotation`) false true)
  (set `CineCameraComponent.FocusSettings` (make `CameraFocusSettings` _focussettings_focusmethod (`KismetMathLibrary.VSize` (- (`SceneComponent.RelativeLocation` _cinecamera) (0.0 0.0 160.0))) _focussettings_trackingfocussettings _focussettings_bsmoothfocuschanges _focussettings_focussmoothinginterpspeed _focussettings_focusoffset) _cinecamera))

(fn `UserConstructionScript`)